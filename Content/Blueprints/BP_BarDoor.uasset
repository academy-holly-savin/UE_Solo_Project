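; BP_BarDoor is a door Blueprint that opens and closes by translating its Hinge component rather than rotating it.
; OpenDoor and CloseDoor each play their own timeline, feeding MoveDoorToLocation with the open or closed location, then call the parent implementation on finish.
; MoveDoorToLocation lerps from the Hinge's current relative location each update, not a stored start, so movement compounds on the timeline curve.
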(event EventOpenDoor
  (bind _increment (Timeline|Timeline PlayFromStart)
    (:Update
      (CallFunction|MoveDoortoLocation (Variables|Default|GetDoorOpenLocation) _increment))
    (:Finished
      (|CallParentFunction))))

(event EventCloseDoor
  (bind _increment (Timeline|Timeline_0 PlayFromStart)
    (:Update
      (CallFunction|MoveDoortoLocation (Variables|Default|GetDoorClosedLocation) _increment))
    (:Finished
      (|CallParentFunction))))

(fn ConstructionScript
  (|CallParentFunction))

(fn MoveDoortoLocation
  (params (EndPosition :type Vector) (PercentComplete :type Float%20%28double-precision%29))
  (bind _hinge (Variables|Default|GetHinge))
  (Transformation|SetRelativeLocation _hinge (Math|Vector|Lerp(Vector) (Variables|/Script/Engine.SceneComponent|GetRelativeLocation _hinge) EndPosition PercentComplete) false false))