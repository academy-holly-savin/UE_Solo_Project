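; Pickup cube that the third-person character collects on touch and that bobs while it is held.
; Box overlap casts to BP_ThirdPersonCharacter and, if that character is not already holding something, calls its PickUp and sets IsHeld.
; While IsHeld, Tick runs Bobbing, which adds a sine of time since creation to the mesh's current relative Z, so the offset accumulates per frame and depends on frame rate.
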(event OnComponentBeginOverlap(Box)
  (params (OverlappedComponent :type Primitive%20Component%20Object%20Reference) (OtherActor :type Actor%20Object%20Reference) (OtherComp :type Primitive%20Component%20Object%20Reference) (OtherBodyIndex :type Integer) (bFromSweep :type Boolean) (SweepResult :type Hit%20Result%20Structure%20%28by%20ref%29))
  ;[1 1 1] Overlap Event
  (bind _asbp_third_person_character (Utilities|Casting|CastToBP_ThirdPersonCharacter OtherActor))
  (if (not (Variables|/Game/ThirdPerson/Blueprints/BP_ThirdPersonCharacter.BP_ThirdPersonCharacter_C|GetIsHolding _asbp_third_person_character))
    (Default|PickUp _asbp_third_person_character self)
    (Variables|Default|SetIsHeld true)))

(event EventBeginPlay)

(event Collision|EventActorBeginOverlap
  (params (OtherActor :type Actor%20Object%20Reference)))

(event EventTick
  (params (DeltaSeconds :type Float%20%28single-precision%29))
  (if (Variables|Default|GetIsHeld)
    (CallFunction|Bobbing)))

(fn ConstructionScript)

(fn Bobbing
  (bind _staticmesh (Variables|Default|GetStaticMesh))
  (bind _relativelocation (Variables|/Script/Engine.SceneComponent|GetRelativeLocation _staticmesh))
  (Transformation|SetRelativeLocation _staticmesh (Math|Vector|MakeVector (.x _relativelocation) (.y _relativelocation) (+ (.z _relativelocation) (* (Math|Trig|Sin(Degrees) (* (Actor|GetGameTimeSinceCreation) (Variables|Default|GetBobbingSpeed))) (Variables|Default|GetBobbingDistance)))) false false))