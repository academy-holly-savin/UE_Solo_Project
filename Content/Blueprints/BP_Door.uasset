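; BP_Door is an interactable door that toggles between open and closed states.
; The Interactwith event checks IsDoorOpen and calls either CloseDoor or OpenDoor.
; Each sets the flag and swaps one DoorFrame material slot to solid green for open or solid red for closed.
; The state change is purely a flag and color indicator, with no movement or collision change in the graph.
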(event Custom|OpenDoor
  (Rendering|Material|SetMaterial (Variables|Default|GetDoorFrame) 2 "/Game/Materials/MI_Solid_Green.MI_Solid_Green")
  (Variables|Default|SetIsDoorOpen true))

(event Custom|CloseDoor
  (Rendering|Material|SetMaterial (Variables|Default|GetDoorFrame) 2 "/Game/Materials/MI_Solid_Red.MI_Solid_Red")
  (Variables|Default|SetIsDoorOpen false))

(event EventInteractwith
  (if (Variables|Default|GetIsDoorOpen)
    (CallFunction|CloseDoor)
    (else
      (CallFunction|OpenDoor))))

(fn ConstructionScript)