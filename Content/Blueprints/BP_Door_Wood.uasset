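; BP_Door_Wood is a wooden door that swings open and closed around its yaw axis.
; OpenDoor and CloseDoor events each play their own timeline toward an open or closed yaw, setting IsDoorOpen when finished.
; Both feed RotateDoor, which lerps from the door's current relative rotation rather than a stored start, so timeline alpha compounds each update.
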(event EventOpenDoor
  (bind _increment (Timeline|Timeline_0 PlayFromStart)
    (:Update
      (CallFunction|RotateDoor (Variables|Default|GetOpenRotationZ) _increment))
    (:Finished
      (Variables|Default|SetIsDoorOpen true))))

(event EventCloseDoor
  (bind _increment (Timeline|Timeline_1 PlayFromStart)
    (:Update
      (CallFunction|RotateDoor (Variables|Default|GetClosedRotationZ) _increment))
    (:Finished
      (Variables|Default|SetIsDoorOpen false))))

(fn ConstructionScript
  (|CallParentFunction))

(fn RotateDoor
  (params (RotationZ :type Float%20%28double-precision%29) (PercentageComplete :type Float%20%28double-precision%29))
  (bind _door (Variables|Default|GetDoor))
  (bind _relativerotation (Variables|/Script/Engine.SceneComponent|GetRelativeRotation _door))
  (Transformation|SetRelativeRotation (Variables|Default|GetDoor) (Math|Rotator|Lerp(Rotator) (Math|Rotator|MakeRotator (.roll _relativerotation) (.pitch _relativerotation) (.yaw _relativerotation)) (Math|Rotator|MakeRotator (.roll _relativerotation) (.pitch _relativerotation) RotationZ) PercentageComplete) false false))