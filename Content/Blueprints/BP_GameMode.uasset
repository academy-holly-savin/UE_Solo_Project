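; Game mode that tracks a trigger-button puzzle and opens the final bar door when no platforms remain.
; On BeginPlay it counts all BP_TriggerButton actors, binds to its count-updated dispatcher and adds WBP_HUD to the viewport.
; PlatformActivated and PlatformDeactivated adjust and broadcast the remaining count; its listener opens BP_BarDoor at zero or below.
; CloseFinalDoor can close the door, but nothing in this graph calls it.
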(event Custom|PlatformDeactivated
  ;[1 1 1] Platform Events
  (bind _result (Math|Integer|IncrementInt (Variables|Default|GetTriggerPlatformsRemaining))
    (:%20%20
      (Default|CallPlatformTriggerCountUpdated _result))))

(event Custom|PlatformTriggerCountUpdated_Event
  (params (Count :type Integer))
  ;[1 1 1] Event Begin
  ;;[1 1 1] Dispatcher Event set up
  (if (<= Count 0)
    (CallFunction|OpenFinalDoor)))

(event Custom|CloseFinalDoor
  ;[1 1 1] Final Door Events
  (bind _returnvalue (Actor|GetActorOfClass "/Game/Blueprints/Doors/BP_BarDoor.BP_BarDoor_C"))
  (Default|CloseDoor _returnvalue))

(event Custom|PlatformActivated
  ;[1 1 1] Platform Events
  (bind _result (Math|Integer|DecrementInt (Variables|Default|GetTriggerPlatformsRemaining))
    (:%20%20
      (Default|CallPlatformTriggerCountUpdated _result))))

(event Custom|OpenFinalDoor
  ;[1 1 1] Final Door Events
  (bind _returnvalue (Actor|GetActorOfClass "/Game/Blueprints/Doors/BP_BarDoor.BP_BarDoor_C"))
  (Default|OpenDoor _returnvalue))

(event EventBeginPlay
  ;[1 1 1] Event Begin
  (Utilities|FlowControl|Sequence
    (:then_0
      ;;[1 1 1] Platform Count
      (bind _outactors (Actor|GetAllActorsOfClass "/Game/Blueprints/BP_TriggerButton.BP_TriggerButton_C"))
      (Variables|Default|SetTriggerPlatformsRemaining (Utilities|Array|Length _outactors)))
    (:then_1
      ;;[1 1 1] Dispatcher Event set up
      (EventDispatchers|BindEventtoPlatformTriggerCountUpdated (delegate Custom|PlatformTriggerCountUpdated_Event))
      (bind _returnvalue (UserInterface|CreateWidget "/Game/UI/WBP_HUD.WBP_HUD_C"))
      (UserInterface|Viewport|AddtoViewport _returnvalue 0))))

(fn ConstructionScript)