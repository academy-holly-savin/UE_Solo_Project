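; BP_ItemSpawner keeps up to MaxItemCount BP_Item actors alive, spawning them at its own transform.
; It spawns one item on BeginPlay, then each Tick prunes invalid references from the Items array and spawns at most one more while below the cap.
; CleanUpItemRefs calls itself recursively after each removal it makes while looping over the array.
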(event EventBeginPlay
  (CallFunction|SpawnItem))

(event EventTick
  (params (DeltaSeconds :type Float%20%28single-precision%29))
  (CallFunction|CleanUpItemRefs)
  (CallFunction|SpawnItem))

(fn ConstructionScript)

(fn SpawnItem
  (if (< (Utilities|Array|Length (Variables|Default|GetItems)) (Variables|Default|GetMaxItemCount))
    (bind _returnvalue (Game|SpawnActorfromClass "/Game/Blueprints/BP_Item.BP_Item_C" (Transformation|GetActorTransform) "Undefined" "MultiplyWithRoot" 0 0))
    (Utilities|Array|Add (Variables|Default|GetItems) _returnvalue)))

(fn CleanUpItemRefs
  (bind _items (Variables|Default|GetItems))
  (for _array_element _items
    (if (not (Utilities|IsValid _array_element))
      (Utilities|Array|RemoveItem _items _array_element)
      (CallFunction|CleanUpItemRefs))))