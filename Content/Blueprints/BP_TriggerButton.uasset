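; BP_TriggerButton is a trigger button that activates and opens a linked door when a BP_Item actor overlaps it.
; On overlap it adds the item to its Cubes array, switches its mesh to a green material and marks itself active.
; It then notifies BP_GameMode through PlatformActivated and calls OpenDoor on its Door reference.
; It has no end-overlap handling, so nothing here reverts the activation.
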(event EventBeginPlay)

(event Collision|EventActorBeginOverlap
  (params (OtherActor :type Actor%20Object%20Reference))
  ;[1 1 1] Overlap Begin
  (bind _asbp_item (Utilities|Casting|CastToBP_Item OtherActor))
  (Utilities|Array|Add (Variables|Default|GetCubes) _asbp_item)
  (Rendering|Material|SetMaterial (Variables|Default|GetStaticMesh) 0 "/Game/Materials/MI_Solid_Green.MI_Solid_Green")
  (Variables|Default|SetActive true)
  (bind _asbp_game_mode (Utilities|Casting|CastToBP_GameMode (Game|GetGameMode)))
  (Default|PlatformActivated _asbp_game_mode)
  (Default|OpenDoor (Variables|Default|GetDoor)))

(event EventTick
  (params (DeltaSeconds :type Float%20%28single-precision%29)))

(fn ConstructionScript)