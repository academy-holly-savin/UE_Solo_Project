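; BP_TriggerPlatform is a trigger platform that activates while BP_Item actors overlap it.
; Overlapping items are tracked in a Cubes array, turning the platform green and active on entry, and red and inactive once the last leaves.
; It reports to BP_ThirdPersonGameMode, calling PlatformActivated on every item entry but PlatformDeactivated only when the array empties.
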(event EventBeginPlay)

(event Collision|EventActorBeginOverlap
  (params (OtherActor :type Actor%20Object%20Reference))
  ;[1 1 1] Overlap Begin
  (bind _asbp_item (Utilities|Casting|CastToBP_Item OtherActor))
  (Utilities|Array|Add (Variables|Default|GetCubes) _asbp_item)
  (Rendering|Material|SetMaterial (Variables|Default|GetStaticMesh) 0 "/Game/Materials/MI_Solid_Green.MI_Solid_Green")
  (Variables|Default|SetActive true)
  (bind _asbp_third_person_game_mode (Utilities|Casting|CastToBP_ThirdPersonGameMode (Game|GetGameMode)))
  (Default|PlatformActivated _asbp_third_person_game_mode))

(event EventTick
  (params (DeltaSeconds :type Float%20%28single-precision%29)))

(event Collision|EventActorEndOverlap
  (params (OtherActor :type Actor%20Object%20Reference))
  (bind _cubes (Variables|Default|GetCubes))
  ;[1 1 1] Overlap End
  (bind _asbp_item (Utilities|Casting|CastToBP_Item OtherActor))
  (if (> (Utilities|Array|FindItem _cubes _asbp_item) -1)
    (Utilities|Array|RemoveIndex _cubes (Utilities|Array|FindItem _cubes _asbp_item))
    (if (not (> (Utilities|Array|Length (Variables|Default|GetCubes)) 0))
      (Rendering|Material|SetMaterial (Variables|Default|GetStaticMesh) 0 "/Game/Materials/MI_Solid_Red.MI_Solid_Red")
      (Variables|Default|SetActive false)
      (bind _asbp_third_person_game_mode (Utilities|Casting|CastToBP_ThirdPersonGameMode (Game|GetGameMode)))
      (Default|PlatformDeactivated _asbp_third_person_game_mode))))

(fn ConstructionScript)