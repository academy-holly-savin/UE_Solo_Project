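; BP_WoodenDoor is a child door Blueprint that swings open and closed on a hinge.
; OpenDoor and CloseDoor call their parent events, then play separate timelines that feed the open or closed yaw into RotateDoor.
; RotateDoor lerps only the Hinge's relative yaw, starting from its current rotation each update rather than a cached start, so the timeline alpha compounds into a non-linear swing.
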(event EventOpenDoor
  (|CallParentFunction)
  (bind _increment (Timeline|Timeline PlayFromStart)
    (:Update
      (CallFunction|RotateDoor (Variables|Default|GetOpenRotationZ) _increment))))

(event EventCloseDoor
  (|CallParentFunction)
  (bind _increment (Timeline|Timeline_0 PlayFromStart)
    (:Update
      (CallFunction|RotateDoor (Variables|Default|GetClosedRotationZ) _increment))))

(fn ConstructionScript
  (|CallParentFunction))

(fn RotateDoor
  (params (RotationZ :type Float%20%28double-precision%29) (PercentageComplete :type Float%20%28double-precision%29))
  (bind _hinge (Variables|Default|GetHinge))
  (bind _relativerotation (Variables|/Script/Engine.SceneComponent|GetRelativeRotation _hinge))
  (Transformation|SetRelativeRotation _hinge (Math|Rotator|Lerp(Rotator) (Math|Rotator|MakeRotator (.roll _relativerotation) (.pitch _relativerotation) (.yaw _relativerotation)) (Math|Rotator|MakeRotator (.roll _relativerotation) (.pitch _relativerotation) RotationZ) PercentageComplete) false false))