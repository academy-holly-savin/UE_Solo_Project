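; BP_DefaultState is the player's default movement state in a state pattern, turning input into calls on the Player.
; On move input it first checks for a new surface and, if found, attaches to the wall with the new gravity and switches to BP_ClimbingState, then applies default movement regardless.
; Jump switches to BP_JumpingState, while the charge-jump input charges a jump on both Triggered and Ongoing.
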(event Input|EnhancedActionEvents|EnhancedInputActionIA_Jump
  (params (ActionValue :type Boolean) (ElapsedSeconds :type Float%20%28double-precision%29) (TriggeredSeconds :type Float%20%28double-precision%29) (InputAction :type Input%20Action%20Object%20Reference :default "/Game/ThirdPerson/Input/Actions/IA_Jump.IA_Jump"))
  (Default|ChangeState (Variables|Default|GetPlayer) "/Game/Blueprints/Interfaces/BP_JumpingState.BP_JumpingState_C"))

(event Input|EnhancedActionEvents|EnhancedInputActionIA_Move
  (params (ActionValue :type Vector%202D%20Structure) (ElapsedSeconds :type Float%20%28double-precision%29) (TriggeredSeconds :type Float%20%28double-precision%29) (InputAction :type Input%20Action%20Object%20Reference :default "/Game/ThirdPerson/Input/Actions/IA_Move.IA_Move"))
  (bind _player (Variables|Default|GetPlayer))
  (Utilities|FlowControl|Sequence
    (:then_0
      (bind (_newgravity _newsurface) (Default|HasPlayerFoundNewSurface? _player))
      (if _newsurface
        (Default|AttachtoWall _player _newgravity)
        (Default|ChangeState _player "/Game/Blueprints/Interfaces/BP_ClimbingState.BP_ClimbingState_C")))
    (:then_1
      (Default|DefaultMovement _player (.x ActionValue) (.y ActionValue)))))

(event Input|EnhancedActionEvents|EnhancedInputActionIA_ChargeJump
  (params (ActionValue :type Boolean) (ElapsedSeconds :type Float%20%28double-precision%29) (TriggeredSeconds :type Float%20%28double-precision%29) (InputAction :type Input%20Action%20Object%20Reference :default "/Game/ThirdPerson/Input/Actions/IA_ChargeJump.IA_ChargeJump"))
  (:Triggered
    (Default|ChargeJump (Variables|Default|GetPlayer) :!label _label))
  (:Ongoing
    (goto _label)))