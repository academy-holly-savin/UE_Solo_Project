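; Slime character Blueprint that animates gravity direction, location and material changes over time.
; Gravity and location events play timelines at a given rate, feeding lerp functions and holding IsTransitioning true until finished.
; A third timeline drives material-instance interpolation, dividing its track value by the clamped input alpha.
; Hit events forward directly to OnHit, and the lerp, interpolation and hit logic live outside these graphs.
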(event Collision|EventHit
  (params (MyComp :type Primitive%20Component%20Object%20Reference) (Other :type Actor%20Object%20Reference) (OtherComp :type Primitive%20Component%20Object%20Reference) (bSelfMoved :type Boolean) (HitLocation :type Vector :default "0, 0, 0") (HitNormal :type Vector :default "0, 0, 0") (NormalImpulse :type Vector :default "0, 0, 0") (Hit :type Hit%20Result%20Structure%20%28by%20ref%29))
  ;[1 1 1] OnHit
  (Class|SlimeCharacter|OnHit))

(event EventApplyLocationTransition
  (params (NewLocation :type Vector%20%28by%20ref%29 :default "0, 0, 0") (PlaybackRate :type Float%20%28single-precision%29))
  ;[1 1 1] Timelines
  (Components|Timeline|SetPlayRate (Variables|Default|GetTL_Location) PlaybackRate)
  (bind _transitionspeed (Timeline|TL_Location PlayFromStart)
    (:Update
      (Variables|Default|SetIsTransitioning true)
      (Class|SlimeCharacter|LerpLocation NewLocation _transitionspeed))
    (:Finished
      (Variables|Default|SetIsTransitioning false))))

(event EventApplyGravityTransition
  (params (NewGravityDirection :type Vector%20%28by%20ref%29 :default "0, 0, 0") (PlaybackRate :type Float%20%28single-precision%29))
  ;[1 1 1] Timelines
  (Components|Timeline|SetPlayRate (Variables|Default|GetTL_Gravity) PlaybackRate)
  (bind _transitionspeed (Timeline|TL_Gravity PlayFromStart)
    (:Update
      (Variables|Default|SetIsTransitioning true)
      (Class|SlimeCharacter|LerpGravity NewGravityDirection _transitionspeed))
    (:Finished
      (Variables|Default|SetIsTransitioning false))))

(event EventSetMaterialOverTime
  (params (NewMaterial :type Material%20Instance%20Object%20Reference) (Alpha :type Float%20%28single-precision%29))
  ;[1 1 1] Timelines
  (bind _duration (Timeline|Timeline_1 PlayFromStart)
    (:Update
      (Class|SlimeCharacter|InterpolateMaterialInstances NewMaterial (/ _duration (Math|Float|Clamp(Float) Alpha))))))

(fn ConstructionScript)