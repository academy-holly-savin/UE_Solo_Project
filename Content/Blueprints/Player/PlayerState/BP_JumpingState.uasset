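; Player state for the slime character's jump, launching it along the mesh's combined forward and up vectors scaled by stored jump velocity.
; Entering consumes that velocity, plays the jump sound and resets the material, while move input keeps driving default movement.
; On hit it attaches to any new surface, then switches to default or climbing, or detaches into falling if nothing is climbable.
; Exiting plays a splat sound.
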(event Input|EnhancedActionEvents|EnhancedInputActionIA_Move
  (params (ActionValue :type Vector%202D%20Structure) (ElapsedSeconds :type Float%20%28double-precision%29) (TriggeredSeconds :type Float%20%28double-precision%29) (InputAction :type Input%20Action%20Object%20Reference :default "/Game/Input/Actions/IA_Move.IA_Move"))
  ;[1 1 1] Handle Movement Input
  (Default|DefaultMovement (Variables|Default|GetPlayer) (.x ActionValue) (.y ActionValue)))

(event EventOnHit
  (bind _player (Variables|Default|GetPlayer))
  (bind _player_2 (Variables|Default|GetPlayer))
  ;[1 1 1] OnHit
  (bind (_newgravity _newsurface) (Default|HasPlayerFoundNewSurface? _player))
  (if _newsurface
    (Default|AttachtoWall _player _newgravity)
    (bind _isgrounded (Default|IsPlayerGrounded? _player_2 :!label _label))
    (if _isgrounded
      (Default|ChangeState _player "/Game/Blueprints/Player/PlayerState/BP_DefaultState.BP_DefaultState_C")
      (else
        (Default|ChangeState _player "/Game/Blueprints/Player/PlayerState/BP_ClimbingState.BP_ClimbingState_C")))
    (else
      (bind _onvalidsurface (Default|IsPlayeronClimableSurface? _player))
      (if _onvalidsurface
        (goto _label)
        (else
          (Default|DetachfromWall _player_2)
          (Default|ChangeState _player_2 "/Game/Blueprints/Player/PlayerState/BP_FallingState.BP_FallingState_C"))))))

(event EventExitState
  ;[1 1 1] OnExit
  (Audio|PlaySoundatLocation "/Game/Audio/Cues/S_SlimeSplat.S_SlimeSplat" (Transformation|GetActorLocation (Variables|Default|GetPlayer)) "0, 0, 0" 1.0 1.0 0.0 0 0 0 0))

(event EventEnterState
  (bind _player (Variables|Default|GetPlayer))
  (bind _player_2 (Variables|Default|GetPlayer))
  (bind _slimemesh (Variables|/Game/Blueprints/Player/BP_ThirdPersonCharacter.BP_ThirdPersonCharacter_C|GetSlimeMesh _player))
  ;[1 1 1] OnEnter
  (Character|LaunchCharacter (Variables|Default|GetPlayer) (* (Variables|/Game/Blueprints/Player/BP_ThirdPersonCharacter.BP_ThirdPersonCharacter_C|GetJumpVelocity (Variables|Default|GetPlayer)) (+ (Math|Vector|GetForwardVector (Transformation|GetWorldRotation _slimemesh)) (Math|Vector|GetUpVector _slimemesh))) false false)
  (Variables|/Game/Blueprints/Player/BP_ThirdPersonCharacter.BP_ThirdPersonCharacter_C|SetJumpVelocity _player_2 (Math|Conversions|ToVector(Float) 0.0))
  (Audio|PlaySoundatLocation "/Game/Audio/Cues/S_Jump.S_Jump" (Transformation|GetActorLocation (Variables|Default|GetPlayer)) "0, 0, 0" 1.0 1.0 0.0 0 0 0 0)
  (Default|ResetMaterial _player_2))