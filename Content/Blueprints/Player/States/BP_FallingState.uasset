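; BP_FallingState is the player state for falling, one state in the player's state machine.
; On entry it clears any non-zero jump velocity and resets the player's material.
; Move input still drives the player's default movement, and each hit checks for ground, switching to BP_DefaultState when grounded.
; Exiting the state plays a slime splat sound at the player's location.
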(event Input|EnhancedActionEvents|EnhancedInputActionIA_Move
  (params (ActionValue :type Vector%202D%20Structure) (ElapsedSeconds :type Float%20%28double-precision%29) (TriggeredSeconds :type Float%20%28double-precision%29) (InputAction :type Input%20Action%20Object%20Reference :default "/Game/Input/Actions/IA_Move.IA_Move"))
  ;[1 1 1] Handle Movement Input
  (Default|DefaultMovement (Variables|Default|GetPlayer) (.x ActionValue) (.y ActionValue)))

(event EventEnterState
  (bind _player (Variables|Default|GetPlayer))
  ;[1 1 1] OnEnter
  (if (Class|KismetMathLibrary|NotEqualExactlyVectorVector (Variables|/Game/Blueprints/Player/BP_ThirdPersonCharacter.BP_ThirdPersonCharacter_C|GetJumpVelocity _player) "0, 0, 0")
    (Variables|/Game/Blueprints/Player/BP_ThirdPersonCharacter.BP_ThirdPersonCharacter_C|SetJumpVelocity _player (Math|Conversions|ToVector(Float) 0.0))
    (Default|ResetMaterial _player)))

(event EventOnHit
  (bind _player (Variables|Default|GetPlayer))
  ;[1 1 1] OnHit
  (bind _isgrounded (Default|IsPlayerGrounded? _player))
  (if _isgrounded
    (Default|ChangeState _player "/Game/Blueprints/Player/States/BP_DefaultState.BP_DefaultState_C")))

(event EventExitState
  ;[1 1 1] OnExit
  (Audio|PlaySoundatLocation "/Game/Audio/Cues/S_SlimeSplat.S_SlimeSplat" (Transformation|GetActorLocation (Variables|Default|GetPlayer)) "0, 0, 0" 1.0 1.0 0.0 0 0 0 0))